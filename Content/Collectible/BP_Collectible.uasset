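; BP_Collectible is a pickup actor that the player collects by touching it.
; On actor overlap, it checks that the other actor is the first player's pawn, then destroys itself.
; The same execution chain then casts the player character to BP_Personnage and increments its NbColl counter, so the count lives on the character.
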(event `self.ReceiveActorBeginOverlap`
  (params (OtherActor :type "Actor Object Reference"))
  (if (== OtherActor (`GameplayStatics.GetPlayerPawn` 0))
    (`self.K2_DestroyActor`)
    (bind _asbp_personnage (cast `/Game/Personnage/BP_Personnage` (`GameplayStatics.GetPlayerCharacter` 0)))
    (bind _asbp_personnage_2 (cast `/Game/Personnage/BP_Personnage` (`GameplayStatics.GetPlayerCharacter` 0)))
    (set `/Game/Personnage/BP_Personnage.nb_Coll` (+ (`/Game/Personnage/BP_Personnage.nb_Coll` _asbp_personnage) 1) _asbp_personnage_2)))

(fn `UserConstructionScript`)