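; Saw trap that moves, spins and damages the player character (BP_Personnage) on contact.
; A Timeline started at BeginPlay offsets the Cube from its cached starting relative location.
; Tick adds a fixed roll increment each frame, so spin speed depends on frame rate.
; Entering the Box trigger calls Degats on BP_Personnage once per overlap, ignoring other actors.
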(event `self.ReceiveBeginPlay`
  ;[1 1 1] Mouvement
  (`|ExecutionSequence`
    (:`then_0`
      (set `self.location_depart` (`SceneComponent.RelativeLocation` (`self.Cube`))))
    (:`then_1`
      (bind (_direction _newtrack_0) (`Timeline|Timeline_1` :`NewTime` 5.0)
        (:`Update`
          (`SceneComponent.K2_SetRelativeLocation` (`self.Cube`) (+ _newtrack_0 (`self.location_depart`)) false false))))))

(event `self.Box.OnComponentBeginOverlap`
  (params (OverlappedComponent :type "PrimitiveComponent Object Reference") (OtherActor :type "Actor Object Reference") (OtherComp :type "PrimitiveComponent Object Reference") (OtherBodyIndex :type Integer) (bFromSweep :type Boolean) (SweepResult :type "HitResult Structure (by ref)"))
  ;[1 1 1] Degats
  (bind _asbp_personnage (cast `/Game/Personnage/BP_Personnage` OtherActor))
  (`/Game/Personnage/BP_Personnage.Degats` _asbp_personnage 1.0))

(event `self.ReceiveTick`
  (params (DeltaSeconds :type "Float (single-precision)"))
  (bind _cube (`self.Cube`))
  (bind (_relativerotation_roll _relativerotation_pitch _relativerotation_yaw) (`KismetMathLibrary.BreakRotator` (`SceneComponent.RelativeRotation` _cube)))
  ;[1 1 1] Rotation
  (`SceneComponent.K2_SetRelativeRotation` _cube (`KismetMathLibrary.MakeRotator` (+ _relativerotation_roll 5.0) _relativerotation_pitch _relativerotation_yaw) false false))

(fn `UserConstructionScript`)