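; BP_Hache is a war axe trap that rotates and damages the player character on overlap.
; On BeginPlay it stores the Cube's starting relative rotation and plays a timeline that lerps the Cube from that rotation toward rotation B.
; When the Box component begins overlapping a BP_Personnage, it calls that character's Degats function with a fixed amount.
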(event `self.ReceiveBeginPlay`
  ;[1 1 1] Deplacement hache
  (`|ExecutionSequence`
    (:`then_0`
      (bind (_direction _newtrack_0) (`Timeline|Timeline_0`)
        (:`Update`
          (`SceneComponent.K2_SetRelativeRotation` (`self.Cube`) (`KismetMathLibrary.RLerp` (`self.rotation depart`) (`self.B`) _newtrack_0) false false))))
    (:`then_1`
      (set `self.rotation depart` (`SceneComponent.RelativeRotation` (`self.Cube`))))))

(event `self.Box.OnComponentBeginOverlap`
  (params (OverlappedComponent :type "PrimitiveComponent Object Reference") (OtherActor :type "Actor Object Reference") (OtherComp :type "PrimitiveComponent Object Reference") (OtherBodyIndex :type Integer) (bFromSweep :type Boolean) (SweepResult :type "HitResult Structure (by ref)"))
  ;[1 1 1] Degats
  (bind _asbp_personnage (cast `/Game/Personnage/BP_Personnage` OtherActor))
  (`/Game/Personnage/BP_Personnage.Degats` _asbp_personnage 1.0))

(fn `UserConstructionScript`)